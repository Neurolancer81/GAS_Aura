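; Firebolt gameplay ability that casts a projectile toward the point under the mouse.
; On activation, mouse target data supplies the location, and the avatar turns to face it through a cached CombatInterface reference.
; It plays the cast montage and waits for the Firebolt montage gameplay event to spawn the projectile at the animation's timing.
; The ability ends after a short delay following the spawn.
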(event `self.K2_ActivateAbility`
  (bind (_asynctaskproxy _datahandle) (`TargetDataUnderMouse.CreateTargetDataUnderMouse`)
    (:`ValidData`
      (set `self.ProjectileTargetLocation` (`.Location` (`GameplayStatics.BreakHitResult` (`AbilitySystemBlueprintLibrary.GetHitResultFromTargetData` _datahandle))))
      (if (not (`KismetSystemLibrary.IsValidInterface` (`self.CombatInterface`)))
        (bind _ascombat_interface (cast `CombatInterface` (`self.GetAvatarActorFromActorInfo`)))
        (bind _output_get (set `self.CombatInterface` _ascombat_interface)))
      (`CombatInterface.UpdateFacingTarget` _output_get (`self.ProjectileTargetLocation`))
      (`AbilityTask_PlayMontageAndWait.CreatePlayMontageAndWaitProxy` "None" "/Game/Assets/Characters/Aura/Animations/Abilities/AM_Cast_FireBolt.AM_Cast_FireBolt"
        (:`then`
          (`AbilityTask_WaitGameplayEvent.WaitGameplayEvent` (struct :`TagName` "Event.Montage.Firebolt") null
            (:`EventReceived`
              (`self.SpawnProjectile` (`self.ProjectileTargetLocation`))
              (`KismetSystemLibrary.Delay` 0.5)
              (`self.K2_EndAbility`))))))))