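; Enemy gameplay ability that performs a ranged attack by spawning a projectile toward the avatar's combat target.
; On activation it turns the avatar to face the target through interface messages and plays a random tagged attack montage.
; A one-time wait for the montage's gameplay event tag times the projectile spawn to the animation.
; The ability ends when the montage completes, is interrupted or is cancelled.
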(event `self.K2_ActivateAbility`
  (bind _output_get (set `self.AvatarActor` (`self.GetAvatarActorFromActorInfo`)))
  (bind _returnvalue (message `EnemyInterface.GetCombatTarget` _output_get))
  (bind _output_get_2 (set `self.ProjectileTargetLocation` (`Actor.K2_GetActorLocation` _returnvalue)))
  (message `CombatInterface.UpdateFacingTarget` (`self.AvatarActor`) _output_get_2)
  (bind _returnvalue_2 (message `CombatInterface.GetAttackMontages` (`self.AvatarActor`)))
  (bind _output_get_3 (set `self.TaggedMontage` (`self.GetRandomTaggedMontageFromArray` _returnvalue_2)))
  (bind (_montage _montagetag) (break `TaggedMontage` _output_get_3))
  (`AbilityTask_PlayMontageAndWait.CreatePlayMontageAndWaitProxy` "None" _montage 1.0 "None" false 1.0 0.0 true
    (:`then`
      (`AbilityTask_WaitGameplayEvent.WaitGameplayEvent` _montagetag null true
        (:`EventReceived`
          (message `CombatInterface.GetCombatSocketLocation` (`self.AvatarActor`) _montagetag)
          (message `EnemyInterface.GetCombatTarget` (`self.AvatarActor`))
          (`self.SpawnProjectile` (`self.ProjectileTargetLocation`)))))
    (:`OnCompleted`
      (`self.K2_EndAbility` :!label _label))
    (:`OnInterrupted`
      (goto _label))
    (:`OnCancelled`
      (goto _label))))