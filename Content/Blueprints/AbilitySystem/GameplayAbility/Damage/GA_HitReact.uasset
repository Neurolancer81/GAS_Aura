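; GA_HitReact is a gameplay ability that plays the avatar's hit-react montage.
; On activation it applies GE_HitReact to the owner and stores the handle, then gets the montage through CombatInterface, caching the avatar cast for reuse.
; The ability ends when the montage completes, is interrupted or is cancelled, and OnEndAbility removes the effect by its stored handle.
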(event `self.K2_ActivateAbility`
  (bind _returnvalue (`self.BP_ApplyGameplayEffectToOwner` "/Game/Blueprints/AbilitySystem/GameplayEffect/Damage/GE_HitReact.GE_HitReact_C"))
  (set `self.ActiveGEHitReact` _returnvalue)
  (if (not (`KismetSystemLibrary.IsValidInterface` (`self.CombatInterface`)))
    (bind _ascombat_interface (cast `CombatInterface` (`self.GetAvatarActorFromActorInfo`)))
    (bind _output_get (set `self.CombatInterface` _ascombat_interface)))
  (bind _returnvalue_2 (`CombatInterface.GetHitReactMontage` _output_get))
  (`AbilityTask_PlayMontageAndWait.CreatePlayMontageAndWaitProxy` "None" _returnvalue_2
    (:`OnCompleted`
      _)
    (:`OnInterrupted`
      _)
    (:`OnCancelled`
      _))
  (`self.K2_EndAbility`))

(event `self.K2_OnEndAbility`
  (params (bWasCancelled :type Boolean))
  (`self.BP_RemoveGameplayEffectFromOwnerWithHandle` (`self.ActiveGEHitReact`)))